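; Friendly spider robot that powers up when the player character touches it, then follows the player.
; The first capsule overlap with BP_ThirdPersonCharacter sets a one-time activation flag and plays the start montage.
; A montage notify marks power-up complete and starts FollowPlayer, a delayed AI MoveTo that re-triggers itself only on success.
; An unconnected, timed random-offset move remains in the graph and never runs.
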(event `ActivateRobotEvent`
  (if (`self.ActivateRobot`)
    (`|PlayMontage` (`self.Mesh`) "/Game/Spider_Robot/Animations/Anim_Start_Montage.Anim_Start_Montage"
      (:`OnNotifyBegin`
        (set `self.RobotPowerUpCompleted` true)
        (`self.Follow Player`)))))

(event `Follow Player`
  (if (`self.RobotPowerUpCompleted`)
    (`KismetSystemLibrary.Delay` 0.5)
    (`|AIMoveTo` self (0.0 0.0 0.0) (`GameplayStatics.GetPlayerCharacter` 0) 150.0
      (:`OnSuccess`
        (`|ExecutionSequence`
          (:`then_1`
            (`self.Follow Player`)))))))

(event `self.Capsule.OnComponentBeginOverlap`
  (params (OverlappedComponent :type "PrimitiveComponent Object Reference") (OtherActor :type "Actor Object Reference") (OtherComp :type "PrimitiveComponent Object Reference") (OtherBodyIndex :type Integer) (bFromSweep :type Boolean) (SweepResult :type "HitResult Structure (by ref)"))
  (cast `/Game/ThirdPerson/Blueprints/BP_ThirdPersonCharacter` OtherActor)
  (if (not (`self.ActivateRobot`))
    (set `self.ActivateRobot` true)
    (`self.ActivateRobotEvent`)))

(fn `UserConstructionScript`)